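; BP_FinalDoor is a door that opens once every CollectableItem in the level has been collected.
; On BeginPlay it counts all CollectableItem actors and opens immediately if none exist.
; Each ItemCollected event, which nothing in this Blueprint calls, decrements that count and triggers OpenDoor at zero.
; Opening destroys the actor and plays a disappearing sound at the world origin rather than at the door.
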(event `self.ReceiveBeginPlay`
  (bind _outactors (`GameplayStatics.GetAllActorsOfClass` "/Game/IA/GamePlayComponents/CollectableItem.CollectableItem_C"))
  (bind _output_get (set `self.RemainingCollectableItem` (`KismetArrayLibrary.Array_Length` _outactors)))
  (if (== _output_get 0)
    (`self.OpenDoor`)))

(event `OpenDoor`
  (`self.K2_DestroyActor`)
  (`GameplayStatics.PlaySoundAtLocation` "/Game/Sonido/sonido-de-desaparecer-made-with-Voicemod-technology.sonido-de-desaparecer-made-with-Voicemod-technology" (0.0 0.0 0.0) (struct) 1.0 1.0 0.0 null null null null))

(event `ItemCollected`
  (bind _result (`/Engine/EditorBlueprintResources/StandardMacros.DecrementInt` (`self.RemainingCollectableItem`))
    (:`  `
      (if (== _result 0)
        (`self.OpenDoor`)))))

(fn `UserConstructionScript`)